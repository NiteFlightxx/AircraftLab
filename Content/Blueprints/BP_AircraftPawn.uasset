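; Quadrotor aircraft pawn that serves as a test rig for the Autopilot and FlightController components, arming on BeginPlay with trajectory debug drawing enabled.
; One thumb button holds slow motion; the other sends Autopilot to a random nearby point at a fixed facing yaw.
; Hard body hits fail all four rotors and raise damping.
; The spring arm scales with the actor; path-following and single-rotor failure experiments are left unwired.
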(event OnComponentHit(BodyMesh)
  (params (HitComponent :type Primitive%20Component%20Object%20Reference) (OtherActor :type Actor%20Object%20Reference) (OtherComp :type Primitive%20Component%20Object%20Reference) (NormalImpulse :type Vector :default "0, 0, 0") (Hit :type Hit%20Result%20Structure%20%28by%20ref%29))
  (bind _bodymesh (Variables|Default|GetBodyMesh))
  (if (> (Math|Vector|VectorLength NormalImpulse) 1e+04)
    (Class|FlightControllerComponent|FailRotors (Variables|Default|GetFlightController) (Utilities|Array|MakeArray 0 1 2 3))
    (Development|PrintString "Fail" true true "(R=1.000000,G=0.000000,B=0.000000,A=1.000000)" 2e+01 "Fail")
    (Class|PrimitiveComponent|SetLinearDamping _bodymesh 3.0)
    (Class|PrimitiveComponent|SetAngularDamping _bodymesh 3.0)))

(event Custom|CustomEvent
  (params (Result :type Autopilot%20Intent%20Result%20Structure%20%28by%20ref%29)))

(event Input|EnhancedActionEvents|EnhancedInputActionIA_AirLook
  (params (ActionValue :type Vector%202D%20Structure) (ElapsedSeconds :type Float%20%28double-precision%29) (TriggeredSeconds :type Float%20%28double-precision%29) (InputAction :type Input%20Action%20Object%20Reference :default "/AircraftLab/Input/IA_AirLook.IA_AirLook"))
  (bind (_x _y) (Math|Vector2D|BreakVector2D ActionValue))
  (Pawn|Input|AddControllerYawInput _x)
  (Pawn|Input|AddControllerPitchInput _y))

(event EventTick
  (params (DeltaSeconds :type Float%20%28single-precision%29))
  (|CallParentFunction DeltaSeconds))

(event EventBeginPlay
  (EventDispatchers|BindEventtoOnIntentFinished (Variables|Default|GetAutopilot) (delegate Custom|CustomEvent))
  (Development|ExecuteConsoleCommand "Autopilot.DebugDrawTrajectory 1" 0)
  (Development|ExecuteConsoleCommand "Autopilot.DebugDrawSetpoint 1" 0)
  (Development|ExecuteConsoleCommand "Autopilot.DebugDrawLookAhead 1" 0)
  (Development|ExecuteConsoleCommand "Autopilot.DebugDrawVelocity 1" 0)
  (Development|ExecuteConsoleCommand "Autopilot.DebugDrawThickness 1" 0)
  (Class|FlightControllerComponent|Arm (Variables|Default|GetFlightController)))

(event Input|MouseEvents|ThumbMouseButton2
  (params (Key :type Key%20Structure :default "None"))
  (:Pressed
    (Variables|Default|SetCurrentPosition (Transformation|GetActorLocation))
    (Variables|Default|SetTargetPosition (Math|Random|RandomPointinBoundingBox (Variables|Default|GetCurrentPosition) "2000.000000,2000.000000,10.000000"))
    (Class|AutopilotComponent|SetAutopilotActive (Variables|Default|GetAutopilot) true)
    (Variables|Default|SetFixed%20Yaw%20Degrees (.yaw (Math|Rotator|MakeRotfromX (- (Variables|Default|GetTargetPosition) (Transformation|GetActorLocation)))))
    (Development|PrintString (Utilities|String|ToString(Float) (.yaw (Math|Rotator|MakeRotfromX (- (Variables|Default|GetTargetPosition) (Transformation|GetActorLocation))))))
    (Class|AutopilotComponent|SubmitMoveto (Variables|Default|GetAutopilot) (Utilities|Struct|MakeAutopilotMoveToCommand (Variables|Default|GetTargetPosition) 0 (Utilities|Struct|MakeAutopilotFiniteCommandOptions (Utilities|Struct|MakeTrajectoryMotionConstraints 8e+02 4e+02) (Utilities|Struct|MakeAutopilotHeadingOptions "FixedYaw" (Variables|Default|GetFixed%20Yaw%20Degrees)) "StopAndComplete" (Utilities|Struct|MakeAutopilotArrivalCriteria 2.0 2.0 1e+01))))))

(event Input|MouseEvents|ThumbMouseButton
  (params (Key :type Key%20Structure :default "None"))
  (:Pressed
    (Utilities|Time|SetGlobalTimeDilation 0.05))
  (:Released
    (Utilities|Time|SetGlobalTimeDilation 1.0)))

(event Input|KeyboardEvents|1
  (params (Key :type Key%20Structure :default "None")))

(fn ConstructionScript
  (bind _springarm (Variables|Default|GetSpringArm))
  (Variables|/Script/Engine.SpringArmComponent|SetTargetArmLength _springarm (* (Variables|/Script/Engine.SpringArmComponent|GetTargetArmLength _springarm) (.x (Transformation|GetActorScale3D)) 0.5)))
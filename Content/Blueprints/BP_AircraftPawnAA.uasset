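; Test pawn for a physics-driven rotor aircraft with an autopilot, flown along a path on a key press.
; ThumbMouseButton2 activates AutopilotComponent and submits the BPNVPath path as a velocity-facing, piecewise-linear follow command; its random target only feeds unwired experiments.
; Other inputs drive camera look, slow motion and a PhysicsConstraint simulation-LOD override; hard body hits print "Fail" and raise damping.
; Arming, rotor-failure and other autopilot command chains are left disconnected.
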(event OnComponentHit(BodyMesh)
  (params (HitComponent :type Primitive%20Component%20Object%20Reference) (OtherActor :type Actor%20Object%20Reference) (OtherComp :type Primitive%20Component%20Object%20Reference) (NormalImpulse :type Vector :default "0, 0, 0") (Hit :type Hit%20Result%20Structure%20%28by%20ref%29))
  (bind _bodymesh (Variables|Default|GetBodyMesh))
  (if (> (Math|Vector|VectorLength NormalImpulse) 1e+04)
    (Development|PrintString "Fail" true true "(R=1.000000,G=0.000000,B=0.000000,A=1.000000)" 2e+01 "Fail")
    (Class|PrimitiveComponent|SetLinearDamping _bodymesh 3.0)
    (Class|PrimitiveComponent|SetAngularDamping _bodymesh 3.0)))

(event Custom|CustomEvent
  (params (Result :type %20Structure%20%28by%20ref%29)))

(event Input|EnhancedActionEvents|EnhancedInputActionIA_AirLook
  (params (ActionValue :type Vector%202D%20Structure) (ElapsedSeconds :type Float%20%28double-precision%29) (TriggeredSeconds :type Float%20%28double-precision%29) (InputAction :type Input%20Action%20Object%20Reference :default "/AircraftLab/Input/IA_AirLook.IA_AirLook"))
  (bind (_x _y) (Math|Vector2D|BreakVector2D ActionValue))
  (Pawn|Input|AddControllerYawInput _x)
  (Pawn|Input|AddControllerPitchInput _y))

(event EventTick
  (params (DeltaSeconds :type Float%20%28single-precision%29)))

(event EventBeginPlay)

(event Input|MouseEvents|ThumbMouseButton2
  (params (Key :type Key%20Structure :default "None"))
  (:Pressed
    (Variables|Default|SetCurrentPosition (Transformation|GetActorLocation))
    (Variables|Default|SetTargetPosition (Math|Random|RandomPointinBoundingBox (Variables|Default|GetCurrentPosition) "2000.000000,2000.000000,10.000000"))
    (CallFunction|SetAutopilotActive (Variables|Default|GetAutopilotComponent) true)
    (Variables|Default|SetFixed%20Yaw%20Degrees (.yaw (Math|Rotator|MakeRotfromX (- (Transformation|GetActorLocation) (Variables|Default|GetTargetPosition)))))
    (CallFunction|SubmitFollowPath (Variables|Default|GetAutopilotComponent) (Utilities|Struct|Make (.NewParam (Default|GetPath (Variables|Default|GetBP_NVPath))) 0 (Utilities|Struct|Make (Utilities|Struct|Make 8e+02 4e+02) (Utilities|Struct|Make 0 0.0) 0 0.0 (Utilities|Struct|Make 5e+01 1e+02))))))

(event Input|MouseEvents|ThumbMouseButton
  (params (Key :type Key%20Structure :default "None"))
  (:Pressed
    (Utilities|Time|SetGlobalTimeDilation 0.05))
  (:Released
    (Utilities|Time|SetGlobalTimeDilation 1.0)))

(event Input|KeyboardEvents|1
  (params (Key :type Key%20Structure :default "None"))
  (bind _simulationlod (Variables|Default|GetSimulationLOD))
  (:Pressed
    (CallFunction|ClearManualDriveModeOverride _simulationlod)
    (bind _returnvalue (CallFunction|SetManualDriveModeOverride _simulationlod 0))
    (Development|PrintString (Utilities|String|ToString(Boolean) _returnvalue))))

(fn ConstructionScript
  (bind _springarm (Variables|Default|GetSpringArm))
  (Variables|/Script/Engine.SpringArmComponent|SetTargetArmLength _springarm (* (Variables|/Script/Engine.SpringArmComponent|GetTargetArmLength _springarm) (.x (Transformation|GetActorScale3D)) 0.5)))